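; Player controller for a networked tabletop grid game that lets players drag tokens across the board and creates the game master HUD locally.
; Left-click picks up a token, and a gated Tick eases it above the hovered actor until release drops it.
; Right-click toggles the HUD's token context menu.
; Moves apply locally on remote clients first, while server events forward spawn, move, physics and lock requests to the GameMode.
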(event Custom|ToggleContextMenu
  (bind _array (Utilities|Array|MakeArray "ObjectTypeQuery2"))
  (bind _gamemasterhud (Variables|References|GetGameMasterHUD))
  (bind _gamemasterhud_2 (Variables|References|GetGameMasterHUD))
  (bind _hitresult (Class|PlayerController|GetHitResultUnderCursorforObjects _array true))
  (bind _contextmenuanchor (Variables|/Game/BattleGrids/UI/WBP_GameMasterHUD.WBP_GameMasterHUD_C|GetContextMenuAnchor _gamemasterhud))
  (bind _contextmenuanchor_2 (Variables|/Game/BattleGrids/UI/WBP_GameMasterHUD.WBP_GameMasterHUD_C|GetContextMenuAnchor _gamemasterhud_2))
  (bind (_bblockinghit _binitialoverlap _time _distance _location _impactpoint _normal _impactnormal _physmat _hitactor) (Collision|BreakHitResult _hitresult))
  (if (Class|MenuAnchor|IsOpen _contextmenuanchor_2)
    (Class|MenuAnchor|Close _contextmenuanchor_2)
    (elif _bblockinghit
      (Utilities|IsValid _hitactor
        (:Is%20Valid
          (bind _asbgtoken (Utilities|Casting|CastToBGToken _hitactor))
          (bind _returnvalue (Class|WidgetLayoutLibrary|GetMousePositiononViewport))
          (Class|CanvasPanelSlot|SetPosition (Class|WidgetLayoutLibrary|SlotasCanvasSlot _contextmenuanchor) _returnvalue)
          (Variables|/Game/BattleGrids/UI/WBP_GameMasterHUD.WBP_GameMasterHUD_C|SetTokenReference _gamemasterhud _asbgtoken)
          (Class|MenuAnchor|Open _contextmenuanchor false))))))

(event EventBeginPlay
  ;[1 1 1] BeginPlay (if local, make a HUD)
  (if (Pawn|IsLocalController)
    (bind _returnvalue (UserInterface|CreateWidget "/Game/BattleGrids/UI/WBP_GameMasterHUD.WBP_GameMasterHUD_C"))
    (bind _output_get (Variables|References|SetGameMasterHUD _returnvalue))
    (UserInterface|Viewport|AddtoViewport _output_get 0)))

(event EventTick
  (params (DeltaSeconds :type Float%20%28single-precision%29))
  (bind _array (Utilities|Array|MakeArray "ObjectTypeQuery2"))
  (bind _hitresult (Class|PlayerController|GetHitResultUnderCursorforObjects _array true))
  (bind _hitactor (Collision|BreakHitResult _hitresult))
  (bind (_origin _boxextent) (Collision|GetActorBounds _hitactor false false))
  (Utilities|FlowControl|Gate true
    (:Exit
      ;[1 1 1] snap token to hovered object
      (Utilities|IsValid _hitactor
        (:Is%20Valid
          (Variables|Default|SetTargetTile (Math|Vector|MakeVector (.x _origin) (.y _origin) (+ (.z _origin) (.z _boxextent))))
          (bind _selectedtoken (Variables|Default|GetSelectedToken)
            (:then
              (CallFunction|MoveTokentoTile(client) (Math|Interpolation|VInterpTo (Transformation|GetActorLocation _selectedtoken) (+ (Variables|Default|GetTargetTile) "0, 0,100.000000") (Utilities|Time|GetWorldDeltaSeconds) 2e+01) _selectedtoken))
            (:else)))))))

(event Input|ActionEvents|InputActionRightClick
  (params (Key :type Key%20Structure :default "None"))
  ;[1 1 1] Right click - toggle context menu
  (:Pressed
    (CallFunction|ToggleContextMenu)))

(event Input|MouseEvents|LeftMouseButton
  (params (Key :type Key%20Structure :default "None"))
  (bind _array (Utilities|Array|MakeArray "ObjectTypeQuery2"))
  (bind _array_2 (Utilities|Array|MakeArray "ObjectTypeQuery2"))
  (bind _gamemasterhud (Variables|References|GetGameMasterHUD))
  (bind _hitresult (Class|PlayerController|GetHitResultUnderCursorforObjects _array_2 true))
  (bind _hitresult_2 (Class|PlayerController|GetHitResultUnderCursorforObjects _array true))
  (bind _contextmenuanchor (Variables|/Game/BattleGrids/UI/WBP_GameMasterHUD.WBP_GameMasterHUD_C|GetContextMenuAnchor _gamemasterhud))
  (bind (_bblockinghit _binitialoverlap _time _distance _location _impactpoint _normal _impactnormal _physmat _hitactor) (Collision|BreakHitResult _hitresult))
  (bind _hitactor_2 (Collision|BreakHitResult _hitresult_2))
  (bind (_origin _boxextent) (Collision|GetActorBounds _hitactor_2 false false))
  ;[1 1 1] Do trace result with left mouse click, and if token is underneath, get reference to it
  (:Pressed
    (if (Class|MenuAnchor|IsOpen _contextmenuanchor)
      (Class|MenuAnchor|Close _contextmenuanchor))
    (if _bblockinghit
      (Utilities|IsValid _hitactor
        (:Is%20Valid
          (bind _asbgtoken (Utilities|Casting|CastToBGToken _hitactor)
            (:then
              (Variables|Default|SetSelectedToken _asbgtoken)
              (CallFunction|SetTokenPhysicsandCollision(server) (Variables|Default|GetSelectedToken) true false "PhysicsOnly")
              (Utilities|FlowControl|Gate true) ; enters at Open
            )
            (:CastFailed
              (Development|PrintString (Utilities|GetDisplayName _hitactor)))))
        (:Is%20Not%20Valid
          (Development|PrintString "No Actor Hit" :!label _label)))
      (else
        (goto _label))))
  (:Released
    (bind _selectedtoken (Variables|Default|GetSelectedToken)
      (:then
        (CallFunction|MoveTokentoTile(client) (+ (Variables|Default|GetTargetTile) "0, 0,50.000000") _selectedtoken)
        (CallFunction|SetTokenPhysicsandCollision(server) (Variables|Default|GetSelectedToken) true true "QueryAndPhysics")
        (Variables|Default|SetTargetTile "0, 0, 0")
        (Variables|Default|SetSelectedToken 0)
        (Utilities|FlowControl|Gate true) ; enters at Close
      )
      (:else))))

(event Custom|ToggleLockTokenInPlace%20%28client%29
  (params (Token :type BG%20Token%20Object%20Reference) (bLock :type Boolean))
  ;[1 1 1] Lock/Unlock token in position on board (called by ContextMenu from GameMasterHUD)
  (CallFunction|ToggleLockTokeninPlace(server) Token bLock))

(event Custom|MoveTokenToTile%20%28server%29
  (params (Location :type Vector) (TokenToMove :type BG%20Token%20Object%20Reference))
  ;[1 1 1] Move token client-side, if remote, and then call server-side movement (if server, just move server-side)
  (bind _gamemode (Class|BPIGameModeBase|GetGameModeReference(Message) (Game|GetGameMode)))
  (Default|MoveTokentoTile _gamemode Location TokenToMove))

(event Custom|SetTokenPhysicsAndCollision%20%28server%29
  (params (Token :type BG%20Token%20Object%20Reference) (bPhysicsOn :type Boolean) (bGravityOn :type Boolean) (CollisionType :type ECollisionEnabled%20Enum :default "NoCollision"))
  ;[1 1 1] Server tells GameMode to call the multicast function off the token for toggling physics and collision
  (bind _gamemode (Class|BPIGameModeBase|GetGameModeReference(Message) (Game|GetGameMode)))
  (Default|SetTokenPhysicsandCollision _gamemode Token bPhysicsOn bGravityOn CollisionType))

(event Custom|SpawnTokenOnTile%20%28server%29
  (params (Location :type Vector) (RowName :type Name))
  ;[1 1 1] Spawn a token server-side
  (bind _gamemode (Class|BPIGameModeBase|GetGameModeReference(Message) (Game|GetGameMode)))
  (Default|SpawnTokenonTile _gamemode Location RowName))

(event Custom|MoveTokenToTile%20%28client%29
  (params (Location :type Vector) (TokenToMove :type BG%20Token%20Object%20Reference))
  ;[1 1 1] Move token client-side, if remote, and then call server-side movement (if server, just move server-side)
  (Networking|SwitchHasAuthority
    (:Authority
      (Development|PrintString "Authority Path"))
    (:Remote
      (Development|PrintString "Remote Path")
      (Transformation|SetActorLocation TokenToMove Location false true)
      (Transformation|SetActorRotation TokenToMove "0, 0, 0" true)))
  (CallFunction|MoveTokentoTile(server) Location TokenToMove))

(event Custom|ToggleLockTokenInPlace%20%28server%29
  (params (Target :type BG%20Token%20Object%20Reference) (bLock :type Boolean))
  ;[1 1 1] Lock/Unlock token in position on board (called by ContextMenu from GameMasterHUD)
  (bind _gamemode (Class|BPIGameModeBase|GetGameModeReference(Message) (Game|GetGameMode)))
  (Default|ToggleLockTokeninPlace _gamemode Target bLock))

(fn ConstructionScript)

(fn GetPlayerControllerReference
  (return self))