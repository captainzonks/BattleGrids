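; BP_PlayerState is the player state for BattleGrids, carrying a PlayerInfo struct that includes the player's name.
; CopyProperties copies PlayerInfo into the new player state, and OverrideWith pulls it back from the old one, so the data survives player state replacement such as travel or reconnection.
; Both events cast to BP_PlayerState and print debug messages, including the player name or a cast failure.
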(event EventCopyProperties
  (params (NewPlayerState :type Player%20State%20Object%20Reference))
  (Development|PrintString "BP_PlayerState: CopyProperties() triggered" true true "(R=0.000000,G=0.660000,B=1.000000,A=1.000000)" 5.0)
  (bind _asbp_player_state (Utilities|Casting|CastToBP_PlayerState NewPlayerState)
    (:then
      (Development|PrintString (Utilities|String|ToString(Text) (.PlayerName (Utilities|Struct|BreakBGPlayerInfo (Variables|Default|GetPlayerInfo)))))
      (Variables|/Script/BattleGrids.BGPlayerState|SetPlayerInfo _asbp_player_state (Variables|Default|GetPlayerInfo)))
    (:CastFailed
      (Development|PrintString "BP_PlayerState: CopyProperties() - Failed to Cast to BP_PlayerState"))))

(event EventOverrideWith
  (params (OldPlayerState :type Player%20State%20Object%20Reference))
  (Development|PrintString "BP_PlayerState: OverrideWith() triggered")
  (bind _asbp_player_state (Utilities|Casting|CastToBP_PlayerState OldPlayerState)
    (:then
      (Development|PrintString (Utilities|String|ToString(Text) (.PlayerName (Utilities|Struct|BreakBGPlayerInfo (Variables|/Script/BattleGrids.BGPlayerState|GetPlayerInfo _asbp_player_state)))))
      (Variables|Default|SetPlayerInfo (Variables|/Script/BattleGrids.BGPlayerState|GetPlayerInfo _asbp_player_state)))
    (:CastFailed
      (Development|PrintString "BP_PlayerState:OverrideWith() - Failed to Cast to BP_PlayerState"))))

(fn ConstructionScript)