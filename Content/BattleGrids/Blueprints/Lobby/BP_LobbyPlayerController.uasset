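; Lobby player controller Blueprint that declares server and client RPCs for player name, color selection, lobby menu updates and the loading screen.
; All RPC events are empty; their former logic remains as disconnected node chains that never run.
; That dead logic polls for PlayerState, loads the saved name from the GameInstance, checks colors through the lobby GameMode and pushes updates to the LobbyMenu widget, which SetupUIOLD creates.
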(event Custom|SetupLobbyMenuWidget%20%28client%29
  (params (ServerName :type Text%20%28by%20ref%29))
  ;[1 1 1] Creates the Lobby Menu widget and adds to viewport
)

(event Custom|ShowLoadingScreen%20%28client%29
  ;[1 1 1] Creates and shows loading screen
)

(event Custom|InitialSetup%20%28client%29
  (params (ServerName :type Text%20%28by%20ref%29))
  ;[1 1 1] INITIAL SETUP (called by Lobby Game Mode after player has logged in and received a Player Controller)
)

(event Custom|AddConnectedPlayerToPlayerList%20%28client%29
  (params (ConnectedPlayersInfo :type Array%20of%20BG%20Player%20Info%20Structures))
  ;[1 1 1] Updates the player list in the client's Lobby Menu widget
)

(event Custom|UpdateServerSidePlayerInfo%20%28server%29
  (params (PlayerInfo :type BG%20Player%20Info%20Structure%20%28by%20ref%29))
  ;[1 1 1] MAIN SERVER UPDATE CALL
)

(event Custom|UpdateLobbyPlayerCount%20%28client%29
  (params (PlayerCount :type Integer))
  ;[1 1 1] Gets client's lobby widget and pushes new player count to it
)

(event Custom|AssignSelectedColor%20%28server%29
  (params (SelectedColor :type Integer) (Color :type Linear%20Color%20Structure))
  ;[1 1 1] Checks availability of color, then if available assigns that color to the player, and updates the server
)

(event Custom|UpdateAvailableColors%20%28client%29
  (params (bAvailableColors :type Array%20of%20Booleans))
  ;[1 1 1] Gets client's lobby widget, and updates the available colors in the color window
)

(event Custom|SetPlayerName%20%28server%29
  (params (Name :type Text%20%28by%20ref%29))
  ;[1 1 1] Receive a new text from the OptionsMenu to set as the Player Name in the PlayerState's PlayerInfo struct
)

(fn ConstructionScript)

(fn SetupUIOLD
  (params (ServerNameText :type Text))
  (Variables|Default|SetbShowMouseCursor true)
  (bind _returnvalue (UserInterface|CreateWidget "/Game/BattleGrids/UI/Lobby/WBP_LobbyMenu.WBP_LobbyMenu_C" self ServerNameText))
  (bind _output_get (Variables|References|SetLobbyMenu _returnvalue))
  (UserInterface|Viewport|AddtoViewport _output_get 0)
  (Input|SetInputModeUIOnly self (Variables|References|GetLobbyMenu) "DoNotLock")
  (return))