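; Lobby game mode for BattleGrids that tracks connected players, color reservations and readiness, then server-travels everyone to the game map.
; PostLogin polls until server info is read from the GameInstance; logins and logouts then rebuild player info from PlayerStates and push it to every lobby controller.
; That refresh sets CanStartGame when all players are ready with colors.
; It also toggles Game Master permissions and shows loading screens before launch.
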(event Custom|UpdateAllConnectedPlayerLobbyWidgets
  ;[1 1 1] Updates all players' Lobby Widgets with new server-side information
  (bind _output_get (Variables|Config|SetPlayerCount (Utilities|Array|Length (Variables|Network|GetAllConnectedPlayers))))
  (if (> _output_get 0)
    (Utilities|Array|Clear (Variables|Config|GetConnectedPlayersInfo))
    (bind _asbp_lobby_game_state_base (Utilities|Casting|CastToBP_Lobby_GameStateBase (Game|GetGameState)))
    (for _array_element (Variables|/Script/Engine.GameStateBase|GetPlayerArray _asbp_lobby_game_state_base)
      (bind _asbp_player_state (Utilities|Casting|CastToBP_PlayerState _array_element)
        (:then
          (Development|PrintString (Utilities|String|ToString(Text) (Utilities|Text|FormatText "Name = {name}" (.PlayerName (Utilities|Struct|BreakBGPlayerInfo (Variables|/Script/BattleGrids.BGPlayerState|GetPlayerInfo _asbp_player_state))))))
          (Utilities|Array|Add (Variables|Config|GetConnectedPlayersInfo) (Variables|/Script/BattleGrids.BGPlayerState|GetPlayerInfo _asbp_player_state)))
        (:CastFailed
          (Development|PrintString "BP_Lobby_GameModeBase: UpdateAllConnectedPlayerLobbyWidgets() - Failed to Cast to BP_PlayerState"))))
    (Development|PrintString (Utilities|String|ToString(Integer) (Utilities|Array|Length (Variables|Config|GetConnectedPlayersInfo))))
    (for _array_element_2 (Variables|Network|GetAllConnectedPlayers)
      (bind _asbp_lobby_player_controller (Utilities|Casting|CastToBP_Lobby_PlayerController _array_element_2)
        (:then
          (Default|AddConnectedPlayertoPlayerList(client) _asbp_lobby_player_controller (Variables|Config|GetConnectedPlayersInfo))
          (Default|UpdateAvailableColors(client) _asbp_lobby_player_controller (Variables|Config|GetbAvailableColors))
          (Default|UpdateLobbyPlayerCount(client) _asbp_lobby_player_controller (Variables|Config|GetPlayerCount)))
        (:CastFailed
          (Development|PrintString "BP_Lobby_GameModeBase: UpdateAllConnectedPlayerLobbyWidgets() - Failed to Cast to BP_Lobby_PlayerController"))))
    (bind _array_element_3 (Utilities|Array|ForEachLoopwithBreak (Variables|Config|GetConnectedPlayersInfo) :!label _label)
      (:LoopBody
        (if (or (== (.A (Math|Color|BreakColor (.PlayerColor (Utilities|Struct|BreakBGPlayerInfo _array_element_3)))) 0.0) (Math|Boolean|NotEqual(Boolean) (.bReady (Utilities|Struct|BreakBGPlayerInfo _array_element_3)) true))
          (Variables|Config|SetbCanStartGame false)
          (goto _label Break)
          (else
            (Variables|Config|SetbCanStartGame true)))))))

(event Custom|StartLoading
  ;[1 1 1] Show loading screen on all connected players, then launch the game
  (for _array_element (Variables|Network|GetAllConnectedPlayers)
    (bind _asbp_lobby_player_controller (Utilities|Casting|CastToBP_Lobby_PlayerController _array_element)
      (:then
        (Default|ShowLoadingScreen(client) _asbp_lobby_player_controller))
      (:CastFailed
        (Development|PrintString "BP_Lobby_GameModeBase: StartLoading() - Failed to Cast to BP_Lobby_PlayerController"))))
  (CallFunction|LaunchGame))

(event Custom|LaunchGame
  ;[1 1 1] Show loading screen on all connected players, then launch the game
  (bind _asbp_game_instance (Utilities|Casting|CastToBP_GameInstance (Game|GetGameInstance))
    (:then
      (Variables|/Game/BattleGrids/Blueprints/BP_GameInstance.BP_GameInstance_C|SetTotalPlayerCount _asbp_game_instance (Variables|Config|GetPlayerCount))
      (Development|ExecuteConsoleCommand "servertravel /Game/BattleGrids/Levels/DefaultGameMap" (Game|GetPlayerController 0)))
    (:CastFailed
      (Development|PrintString "BP_Lobby_GameModeBase: LaunchGame() - Failed to Cast to BP_GameInstance"))))

(event Custom|SetPlayerPermissions
  (params (PlayerID :type Integer))
  ;[1 1 1] Toggles Game Master permissions on player
  (bind _asbp_lobby_player_controller (Utilities|Casting|CastToBP_Lobby_PlayerController (Utilities|Array|Get(acopy) (Variables|Network|GetAllConnectedPlayers) PlayerID))
    (:then
      (bind _asbp_player_state (Utilities|Casting|CastToBP_PlayerState (Variables|/Script/Engine.Controller|GetPlayerState _asbp_lobby_player_controller))
        (:then
          (bind _structout (Utilities|Struct|SetmembersinBGPlayerInfo (Variables|/Script/BattleGrids.BGPlayerState|GetPlayerInfo _asbp_player_state) (not (.bGameMasterPermissions (Utilities|Struct|BreakBGPlayerInfo (Variables|/Script/BattleGrids.BGPlayerState|GetPlayerInfo _asbp_player_state))))))
          (Default|UpdateServerSidePlayerInfo(server) _asbp_lobby_player_controller _structout))
        (:CastFailed
          (Development|PrintString "BP_Lobby_GameModeBase: SetPlayerPermissions() - Failed to Cast to BP_PlayerState"))))
    (:CastFailed
      (Development|PrintString "BP_Lobby_GameModeBase: SetPlayerPermissions() - Failed to Cast to BP_Lobby_PlayerController"))))

(event Custom|InitializeServerInfo
  (bind _asbp_game_instance (Utilities|Casting|CastToBP_GameInstance (Game|GetGameInstance))
    (:then
      (Variables|Config|SetServerName (Variables|/Game/BattleGrids/Blueprints/BP_GameInstance.BP_GameInstance_C|GetServerName _asbp_game_instance))
      (Variables|Config|SetPlayerCount (Variables|/Game/BattleGrids/Blueprints/BP_GameInstance.BP_GameInstance_C|GetMaxPlayers _asbp_game_instance))
      (Variables|Config|SetbServerInfoReady true))
    (:CastFailed
      (Development|PrintString "BP_Lobby_GameModeBase: BeginPlay() - Failed to Cast to BP_GameInstance"))))

(event EventBeginPlay
  (CallFunction|InitializeServerInfo))

(event EventPostLogin
  (params (NewPlayer :type Player%20Controller%20Object%20Reference))
  ;[1 1 1] Called when Player connects and receives a PlayerController
  (bind _output_get (Variables|Network|SetNewlyConnectedPlayer NewPlayer))
  (Utilities|Array|AddUnique (Variables|Network|GetAllConnectedPlayers) _output_get)
  (bind _asbp_lobby_player_controller (Utilities|Casting|CastToBP_Lobby_PlayerController (Variables|Network|GetNewlyConnectedPlayer))
    (:then
      ;;[1 1 1] Wait for Server to get info
      (if (Variables|Config|GetbServerInfoReady) :!label _label
        (Default|InitialSetup(client) _asbp_lobby_player_controller (Variables|Config|GetServerName))
        (Utilities|FlowControl|Delay 1.0)
        (CallFunction|UpdateAllConnectedPlayerLobbyWidgets)
        (else
          (Utilities|FlowControl|Delay 0.2)
          (goto _label))))
    (:CastFailed
      (Development|PrintString "BP_Lobby_GameModeBase: OnPostLogin() - Failed to Cast to BP_Lobby_PlayerController"))))

(event EventOnLogout
  (params (ExitingController :type Controller%20Object%20Reference))
  ;[1 1 1] Removes connected player information from data arrays and frees up their color for selection, then updates all connected players' lobby widgets
  (bind (_array_element _array_index) (Utilities|Array|ForEachLoopwithBreak (Variables|Network|GetAllConnectedPlayers) :!label _label)
    (:LoopBody
      (if (== _array_element ExitingController)
        (bind _asbp_lobby_player_controller (Utilities|Casting|CastToBP_Lobby_PlayerController _array_element)
          (:then
            (Utilities|Array|SetArrayElem (Variables|Config|GetbAvailableColors) (Variables|/Game/BattleGrids/Blueprints/Lobby/BP_Lobby_PlayerController.BP_Lobby_PlayerController_C|GetSelectedColorID _asbp_lobby_player_controller) false)
            (Utilities|Array|RemoveIndex (Variables|Network|GetAllConnectedPlayers) _array_index)
            (Utilities|Array|RemoveIndex (Variables|Config|GetConnectedPlayersInfo) _array_index)
            (goto _label Break))
          (:CastFailed
            (Development|PrintString "BP_Lobby_GameModeBase: OnLogout() - Failed to Cast to BP_Lobby_PlayerController")))))
    (:Completed
      (CallFunction|UpdateAllConnectedPlayerLobbyWidgets))))

(fn ConstructionScript)

(fn CheckColorAvailability
  (params (SelectedColorID :type Integer) (PreviousColorID :type Integer))
  (bind _bavailablecolors (Variables|Config|GetbAvailableColors))
  (if (Utilities|Array|Get(acopy) (Variables|Config|GetbAvailableColors) SelectedColorID) ; true == unavailable
    (return false)
    (else
      (Utilities|Array|SetArrayElem _bavailablecolors SelectedColorID true)
      (Utilities|Array|SetArrayElem _bavailablecolors PreviousColorID false)
      (return true))))