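; Player controller for the multiplayer lobby that links each client's lobby menu to the Lobby Game Mode.
; Client RPCs build the menu in UI-only input mode, refresh its player list, count and available colors, and swap in a loading screen.
; Server RPCs check color picks with the game mode, mark the player ready and trigger lobby widget updates for everyone.
; Game Instance player info load and save logic is not wired up.
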(event Custom|LoadPlayerInfo
  (bind _gameinstance (Class|BPIGameInstance|GetGameInstanceReference(Message) (Game|GetGameInstance)))
  (bind (_bsuccess _playerinfo) (Class|BPIGameInstance|LoadPlayerInfo(Message) _gameinstance))
  (if _bsuccess
    (bind _structout (Utilities|Struct|SetmembersinBGPlayerInfo _playerinfo "(R=0.000000,G=0.000000,B=0.000000,A=0.000000)"))
    (Variables|Default|SetPlayerInfo _structout)))

(event Custom|SetupLobbyMenuWidget%20%28client%29
  (params (ServerName :type Text))
  ;[1 1 1] Creates the Lobby Menu widget and adds to viewport
  (CallFunction|SetupUI ServerName))

(event Custom|ShowLoadingScreen%20%28client%29
  ;[1 1 1] Creates and shows loading screen
  (bind _lobbymenu (Variables|References|GetLobbyMenu)
    (:then
      (Widget|RemovefromParent _lobbymenu)
      (bind _returnvalue (UserInterface|CreateWidget "/Game/BattleGrids/UI/WBP_LoadingScreen.WBP_LoadingScreen_C" self))
      (UserInterface|Viewport|AddtoViewport _returnvalue 0))
    (:else)))

(event Custom|InitialSetup%20%28client%29
  (params (ServerName :type Text))
  ;[1 1 1] INITIAL SETUP (called by Lobby Game Mode after player has logged in and received a Player Controller)
  (CallFunction|SetupLobbyMenuWidget(client) ServerName))

(event Custom|AddConnectedPlayerToPlayerList%20%28client%29
  (params (ConnectedPlayersInfo :type Array%20of%20BG%20Player%20Info%20Structures))
  (bind _lobbymenu (Variables|References|GetLobbyMenu))
  ;[1 1 1] Updates the player list in the client's Lobby Menu widget
  (bind _lobbymenu_2 (Variables|References|GetLobbyMenu)
    (:then
      (Default|ClearPlayerList _lobbymenu_2)
      (for _array_element ConnectedPlayersInfo
        (Default|AddPlayertoPlayerList _lobbymenu _array_element)
        (Default|PopulateSettingsPlayerList (Variables|/Game/BattleGrids/UI/Lobby/WBP_LobbyMenu.WBP_LobbyMenu_C|GetSettingsWindow _lobbymenu) ConnectedPlayersInfo)))
    (:else)))

(event Custom|UpdateServerSidePlayerInfo%20%28server%29
  (params (PlayerInfo :type BG%20Player%20Info%20Structure))
  ;[1 1 1] MAIN SERVER UPDATE CALL
  (Variables|Default|SetPlayerInfo PlayerInfo)
  (bind _lobbygamemode (Class|BPILobbyGameModeBase|GetLobbyGameModeReference(Message) (Game|GetGameMode)))
  (Default|UpdateAllConnectedPlayerLobbyWidgets _lobbygamemode))

(event Custom|UpdateLobbyPlayerCount%20%28client%29
  (params (PlayerCount :type Integer))
  ;[1 1 1] Gets client's lobby widget and pushes new player count to it
  (Default|UpdatePlayerCount (Variables|References|GetLobbyMenu) PlayerCount))

(event Custom|AssignSelectedColor%20%28server%29
  (params (SelectedColor :type Integer) (Color :type Linear%20Color%20Structure))
  ;[1 1 1] Checks availability of color, then if available assigns that color to the player, and updates the server
  (Variables|Config|SetPreviousColorID (Variables|Config|GetSelectedColorID))
  (Variables|Config|SetSelectedColorID SelectedColor)
  (bind _lobbygamemode (Class|BPILobbyGameModeBase|GetLobbyGameModeReference(Message) (Game|GetGameMode)))
  (bind _bavailable (Default|CheckColorAvailability _lobbygamemode (Variables|Config|GetSelectedColorID) (Variables|Config|GetPreviousColorID)))
  (if _bavailable
    (bind _structout (Utilities|Struct|SetmembersinBGPlayerInfo (Variables|Default|GetPlayerInfo) Color true))
    (CallFunction|UpdateServerSidePlayerInfo(server) _structout)))

(event Custom|UpdateAvailableColors%20%28client%29
  (params (bAvailableColors :type Array%20of%20Booleans))
  ;[1 1 1] Gets client's lobby widget, and updates the available colors in the color window
  (Default|UpdateAvailableColors (Variables|References|GetLobbyMenu) bAvailableColors))

(fn ConstructionScript)

(fn SetupUI
  (params (ServerNameText :type Text))
  (Variables|Default|SetbShowMouseCursor true)
  (bind _returnvalue (UserInterface|CreateWidget "/Game/BattleGrids/UI/Lobby/WBP_LobbyMenu.WBP_LobbyMenu_C" self ServerNameText))
  (bind _output_get (Variables|References|SetLobbyMenu _returnvalue))
  (UserInterface|Viewport|AddtoViewport _output_get 0)
  (Input|SetInputModeUIOnly self (Variables|References|GetLobbyMenu) "DoNotLock"))

(fn GetLobbyPlayerControllerReference
  (return self))