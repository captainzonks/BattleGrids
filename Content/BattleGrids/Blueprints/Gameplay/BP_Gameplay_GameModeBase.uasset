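; Gameplay game mode for BattleGrids that manages player controllers as they join and leave a session.
; Controllers arriving through OnSwapPlayerControllers are added uniquely to ConnectedPlayers.
; HandleStartingNewPlayer has each gameplay PlayerController run its SpawnServer call.
; On logout it passes the exiting controller to the GameInstance's DestroySessionCallerMessage, then removes it from ConnectedPlayers.
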(event EventHandleStartingNewPlayer
  (params (NewPlayer :type Player%20Controller%20Object%20Reference))
  ;[1 1 1] Get the incoming PlayerController, add it to an array, and then spawn
  (bind _asbp_gameplay_player_controller (Utilities|Casting|CastToBP_Gameplay_PlayerController NewPlayer)
    (:then
      (Default|Spawn(server) _asbp_gameplay_player_controller))
    (:CastFailed
      (Development|PrintString "BP_Gameplay_GameModeBase: HandleStartingNewPlayer() - Failed to Cast to BP_Gameplay_PlayerController"))))

(event EventOnLogout
  (params (ExitingController :type Controller%20Object%20Reference))
  (bind _connectedplayers (Variables|Default|GetConnectedPlayers))
  ;[1 1 1] Called when a Controller disconnects
  (bind _asbp_gameplay_player_controller (Utilities|Casting|CastToBP_Gameplay_PlayerController ExitingController)
    (:then
      (bind _asbp_game_instance (Utilities|Casting|CastToBP_GameInstance (Game|GetGameInstance))
        (:then
          (Class|BPIGameInstance|DestroySessionCaller(Message) _asbp_game_instance _asbp_gameplay_player_controller)
          (Utilities|Array|RemoveIndex _connectedplayers (Utilities|Array|FindItem _connectedplayers _asbp_gameplay_player_controller)))
        (:CastFailed
          (Development|PrintString "BP_Gameplay_GameModeBase: OnLogout() - Failed to Cast to BP_GameInstance"))))
    (:CastFailed
      (Development|PrintString "BP_Gameplay_GameModeBase: OnLogout() - Failed to Cast to BP_Gameplay_PlayerController"))))

(event EventOnSwapPlayerControllers
  (params (OldPC :type Player%20Controller%20Object%20Reference) (NewPC :type Player%20Controller%20Object%20Reference))
  ;[1 1 1] Get the incoming PlayerController, add it to an array, and then spawn
  (Utilities|Array|AddUnique (Variables|Default|GetConnectedPlayers) NewPC))

(fn ConstructionScript)