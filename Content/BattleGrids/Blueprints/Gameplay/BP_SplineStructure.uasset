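; BP_SplineStructure is a construction-time actor that lays copies of a configurable static mesh along a spline.
; The construction script assigns the mesh and a fixed polished marble material, then rebuilds the instanced static mesh's instances.
; Straight-line distances between spline points set instance counts, while a running counter places half-scale, spline-aligned instances at fixed intervals.
; MaterialReference only gates the rebuild and is never applied.
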(event EventBeginPlay)

(event Collision|EventActorBeginOverlap
  (params (OtherActor :type Actor%20Object%20Reference)))

(event EventTick
  (params (DeltaSeconds :type Float%20%28single-precision%29)))

(fn ConstructionScript
  (bind _instancedstaticmesh (Variables|Default|GetInstancedStaticMesh))
  (Components|StaticMesh|SetStaticMesh _instancedstaticmesh (Variables|Default|GetStaticMeshReference))
  (Rendering|Material|SetMaterial _instancedstaticmesh 0 "/Game/BattleGrids/Materials/MI_Rock_Marble_Polished.MI_Rock_Marble_Polished")
  (CallFunction|AddInstancedMeshtoSpline))

(fn AddInstancedMeshtoSpline
  (bind _splinecomponent (Variables|Default|GetSplineComponent))
  (Components|InstancedStaticMesh|ClearInstances (Variables|Default|GetInstancedStaticMesh))
  (Utilities|IsValid (Variables|Default|GetStaticMeshReference)
    (:Is%20Valid
      (Utilities|IsValid (Variables|Default|GetMaterialReference)
        (:Is%20Valid
          (LocalVariables|SetLoopCount 0)
          (for _index (range 0 (- (Spline|GetNumberOfSplinePoints _splinecomponent) 2))
            (for _index_2 (range 0 (.ReturnValue (Math|Float|Division(WholeandRemainder) (Math|Vector|Distance(Vector) (Spline|GetLocationatSplinePoint _splinecomponent _index "Local") (Spline|GetLocationatSplinePoint _splinecomponent (+ _index 1) "Local")) 1e+02)))
              (Components|InstancedStaticMesh|AddInstance (Variables|Default|GetInstancedStaticMesh) (Math|Transform|MakeTransform (Math|Vector|MakeVector (.X (Math|Vector|BreakVector (Spline|GetLocationatDistanceAlongSpline _splinecomponent (* (LocalVariables|GetLoopCount) 105.0) "Local"))) (.Y (Math|Vector|BreakVector (Spline|GetLocationatDistanceAlongSpline _splinecomponent (* (LocalVariables|GetLoopCount) 105.0) "Local"))) (.Z (Math|Vector|BreakVector (Spline|GetLocationatDistanceAlongSpline _splinecomponent (* (LocalVariables|GetLoopCount) 105.0) "Local")))) (Math|Rotator|MakeRotator (.Roll (Math|Rotator|BreakRotator (Spline|GetRotationatDistanceAlongSpline _splinecomponent (* (LocalVariables|GetLoopCount) 105.0) "Local"))) (.Pitch (Math|Rotator|BreakRotator (Spline|GetRotationatDistanceAlongSpline _splinecomponent (* (LocalVariables|GetLoopCount) 105.0) "Local"))) (.Yaw (Math|Rotator|BreakRotator (Spline|GetRotationatDistanceAlongSpline _splinecomponent (* (LocalVariables|GetLoopCount) 105.0) "Local")))) "0.500000,0.500000,0.500000"))
              (Math|Integer|IncrementInt (LocalVariables|GetLoopCount)))))))))