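; Player controller for BattleGrids gameplay, handling pawn spawning, game master checks and object bank requests.
; On possess, a server event requests Character and Actor row names from the game mode, then sets game-only input.
; A server Spawn event replaces the pawn with a BP_Pawn at a random PlayerStart.
; Helpers read game master permission from BP_PlayerState and sort actors into token, board or spline structure; older HUD and context-menu logic is disconnected.
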(event Custom|ToggleContextMenu_old
  ;[1 1 1] Toggles a ContextMenu with the object that is right-clicked
)

(event EventPossess
  (params (PossessedPawn :type Pawn%20Object%20Reference))
  ;[1 1 1] SetupUI() after getting a Pawn
  (CallFunction|GetBankDatafromServer(server)))

(event Input|ActionEvents|InputActionContext
  (params (Key :type Key%20Structure :default "None"))
  ;[1 1 1] Toggles a ContextMenu with the object that is right-clicked
)

(event Custom|GetBankDataFromServer%20%28server%29
  ;[1 1 1] Sets up UI : GM HUD if permission found, otherwise Player HUD
  (Development|PrintString "BP_Gameplay_PlayerController: SetupUI() triggered")
  (Class|BGGamePlayerController|GetRowNamesOfObjectTypefromGameMode (Utilities|Enum|LiteralenumEBGClassCategory "Character"))
  (Class|BGGamePlayerController|GetRowNamesOfObjectTypefromGameMode (Utilities|Enum|LiteralenumEBGClassCategory "Actor"))
  (Input|SetInputModeGameOnly self))

(event Custom|Spawn%20%28server%29
  (bind _returnvalue (Pawn|GetControlledPawn))
  ;[1 1 1] Spawn a BP_Pawn and possess it at a random start location
  (Development|PrintString "BP_Gameplay_PlayerController: Spawn() triggered")
  (bind _outactors (Actor|GetAllActorsOfClass "/Script/Engine.PlayerStart"))
  (Utilities|IsValid _returnvalue
    (:Is%20Valid
      (Actor|DestroyActor _returnvalue))
    (:Is%20Not%20Valid
      _))
  (bind _returnvalue_2 (Game|SpawnActorfromClass "/Game/BattleGrids/Blueprints/Gameplay/BP_Pawn.BP_Pawn_C" (Math|Transform|MakeTransform (Transformation|GetActorLocation (Utilities|Array|Get(acopy) _outactors (Math|Random|RandomIntegerinRange 0 (- (Utilities|Array|Length _outactors) 1)))) "0, 0, 0" "1,1,1") "AdjustIfPossibleButAlwaysSpawn" self 0))
  (Pawn|Possess self _returnvalue_2))

(fn ConstructionScript)

(fn IsPlayerGameMaster
  (bind _asbp_player_state (Utilities|Casting|CastToBP_PlayerState (Variables|Default|GetPlayerState))
    (:then
      (return (.bGameMasterPermissions (Utilities|Struct|BreakBGPlayerInfo (Variables|/Script/BattleGrids.BGPlayerState|GetPlayerInfo _asbp_player_state)))))
    (:CastFailed
      (Development|PrintString "BP_Gameplay_PlayerController: DoesPlayerHavePermissions() - Failed to Cast to BP_PlayerState"))))