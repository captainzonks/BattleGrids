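; Gameplay player controller for BattleGrids that handles pawn spawning, role-based HUDs and menus.
; A server event replaces the current pawn with a BP_Pawn at a random PlayerStart.
; Possession triggers client UI setup, which retries until PlayerState exists, then shows the Game Master or player HUD by permission.
; Input toggles a pause menu and the GM HUD's context menu, which targets the actor and item under the cursor.
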(event Custom|ToggleContextMenu
  (bind _array (Utilities|Array|MakeArray "ObjectTypeQuery1" "ObjectTypeQuery2"))
  (bind _gamemasterhud (Variables|References|GetGameMasterHUD))
  (bind _hitresult (Class|PlayerController|GetHitResultUnderCursorforObjects _array true))
  (bind _contextmenuanchor (Variables|/Game/BattleGrids/UI/Gameplay/WBP_GameMasterHUD.WBP_GameMasterHUD_C|GetContextMenuAnchor _gamemasterhud))
  (bind (_bblockinghit _binitialoverlap _time _distance _location _impactpoint _normal _impactnormal _physmat _hitactor _hitcomponent _hitbonename _hititem) (Collision|BreakHitResult _hitresult))
  ;[1 1 1] Toggles a ContextMenu with the object that is right-clicked
  (bind _gamemasterhud_2 (Variables|References|GetGameMasterHUD)
    (:then
      (if (Class|MenuAnchor|IsOpen (Variables|/Game/BattleGrids/UI/Gameplay/WBP_GameMasterHUD.WBP_GameMasterHUD_C|GetContextMenuAnchor _gamemasterhud_2))
        (Class|MenuAnchor|Close (Variables|/Game/BattleGrids/UI/Gameplay/WBP_GameMasterHUD.WBP_GameMasterHUD_C|GetContextMenuAnchor _gamemasterhud_2))
        (elif _bblockinghit
          (Utilities|IsValid _hitactor
            (:Is%20Valid
              (bind _returnvalue (Class|WidgetLayoutLibrary|GetMousePositiononViewport))
              (Class|CanvasPanelSlot|SetPosition (Class|WidgetLayoutLibrary|SlotasCanvasSlot _contextmenuanchor) _returnvalue)
              (Variables|/Game/BattleGrids/UI/Gameplay/WBP_GameMasterHUD.WBP_GameMasterHUD_C|SetContextObjectReference _gamemasterhud _hitactor)
              (Variables|/Game/BattleGrids/UI/Gameplay/WBP_GameMasterHUD.WBP_GameMasterHUD_C|SetContextObjectIndex _gamemasterhud _hititem)
              (Class|MenuAnchor|Open _contextmenuanchor true))))))
    (:else)))

(event EventPossess
  (params (PossessedPawn :type Pawn%20Object%20Reference))
  ;[1 1 1] SetupUI() after getting a Pawn
  (CallFunction|SetupUI(client)))

(event Input|ActionEvents|InputActionContext
  (params (Key :type Key%20Structure :default "None"))
  ;[1 1 1] Toggles a ContextMenu with the object that is right-clicked
  (:Pressed
    (CallFunction|ToggleContextMenu)))

(event Custom|SetupUI%20%28client%29
  (bind _self self)
  (bind _self_2 self)
  ;[1 1 1] Sets up UI : GM HUD if permission found, otherwise Player HUD
  (Development|PrintString "BP_Gameplay_PlayerController: SetupUI() triggered")
  (bind _playerstate (Variables|Default|GetPlayerState :!label _label)
    (:then
      (bind _asbp_player_state (Utilities|Casting|CastToBP_PlayerState _playerstate)
        (:then
          (Viewport|RemoveAllWidgets)
          (if (Utilities|Struct|BreakBGPlayerInfo (Variables|/Script/BattleGrids.BGPlayerState|GetPlayerInfo _asbp_player_state))
            (Variables|References|GetGameMasterHUD
              (:then
                _)
              (:else
                (bind _returnvalue (UserInterface|CreateWidget "/Game/BattleGrids/UI/Gameplay/WBP_GameMasterHUD.WBP_GameMasterHUD_C" _self))
                (bind _output_get (Variables|References|SetGameMasterHUD _returnvalue))))
            (UserInterface|Viewport|AddtoViewport _output_get 0)
            (Input|SetInputModeGameandUI _self_2 _output_get "DoNotLock" false)
            (else
              (Variables|References|GetPlayerHUD
                (:then
                  _)
                (:else
                  (bind _returnvalue_2 (UserInterface|CreateWidget "/Game/BattleGrids/UI/Gameplay/WBP_PlayerHUD.WBP_PlayerHUD_C" _self))
                  (bind _output_get_2 (Variables|References|SetPlayerHUD _returnvalue_2))))
              (UserInterface|Viewport|AddtoViewport _output_get_2 0)
              (Input|SetInputModeGameandUI _self_2 _output_get_2 "DoNotLock" false))))
        (:CastFailed
          (Development|PrintString "BP_Gameplay_PlayerController: SetupUI() - Failed to Cast to BP_PlayerState"))))
    (:else
      (Utilities|FlowControl|Delay 0.5)
      (goto _label))))

(event Custom|Spawn%20%28server%29
  (bind _returnvalue (Pawn|GetControlledPawn))
  ;[1 1 1] Spawn a BP_Pawn and possess it at a random start location
  (Development|PrintString "BP_Gameplay_PlayerController: Spawn() triggered")
  (bind _outactors (Actor|GetAllActorsOfClass "/Script/Engine.PlayerStart"))
  (Utilities|IsValid _returnvalue
    (:Is%20Valid
      (Actor|DestroyActor _returnvalue))
    (:Is%20Not%20Valid
      _))
  (bind _returnvalue_2 (Game|SpawnActorfromClass "/Game/BattleGrids/Blueprints/Gameplay/BP_Pawn.BP_Pawn_C" (Transformation|GetActorTransform (Utilities|Array|Get(acopy) _outactors (Math|Random|RandomIntegerinRange 0 (- (Utilities|Array|Length _outactors) 1)))) "AdjustIfPossibleButAlwaysSpawn" self 0))
  (Pawn|Possess self _returnvalue_2))

(event Custom|TogglePauseMenu
  ;[1 1 1] Toggle Pause Menu
  (bind _pausemenu (Variables|References|GetPauseMenu)
    (:then
      (if (Widget|IsVisible _pausemenu)
        (Widget|SetVisibility (Variables|References|GetPauseMenu) "Hidden")
        (else
          (Widget|SetVisibility (Variables|References|GetPauseMenu) "Visible"))))
    (:else
      (bind _returnvalue (UserInterface|CreateWidget "/Game/BattleGrids/UI/Gameplay/WBP_PauseMenu.WBP_PauseMenu_C" self))
      (bind _output_get (Variables|References|SetPauseMenu _returnvalue))
      (UserInterface|Viewport|AddtoViewport _output_get 0))))

(event Input|ActionEvents|InputActionPauseMenu
  (params (Key :type Key%20Structure :default "None"))
  ;[1 1 1] Toggle Pause Menu
  (:Pressed
    (CallFunction|TogglePauseMenu)))

(fn ConstructionScript)

(fn IsPlayerGameMaster
  (bind _asbp_player_state (Utilities|Casting|CastToBP_PlayerState (Variables|Default|GetPlayerState))
    (:then
      (return (.bGameMasterPermissions (Utilities|Struct|BreakBGPlayerInfo (Variables|/Script/BattleGrids.BGPlayerState|GetPlayerInfo _asbp_player_state)))))
    (:CastFailed
      (Development|PrintString "BP_Gameplay_PlayerController: DoesPlayerHavePermissions() - Failed to Cast to BP_PlayerState"))))