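; Gameplay game mode for BattleGrids, providing a lookup of mesh and material assets by name.
; GetDataFromBank reads the static mesh and material instance data tables by row name and returns both assets, with success only if both are valid.
; New-player handling only calls the parent; the swap and logout events are empty.
; Older logic for spawning, controller tracking and session teardown remains disconnected and never runs.
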(event EventHandleStartingNewPlayer
  (params (NewPlayer :type Player%20Controller%20Object%20Reference))
  ;[1 1 1] Get the incoming PlayerController, add it to an array, and then spawn
  (|CallParentFunction NewPlayer))

(event EventOnLogout
  (params (ExitingController :type Controller%20Object%20Reference))
  ;[1 1 1] Called when a Controller disconnects
)

(event EventOnSwapPlayerControllers
  (params (OldPC :type Player%20Controller%20Object%20Reference) (NewPC :type Player%20Controller%20Object%20Reference))
  ;[1 1 1] Get the incoming PlayerController, add it to an array, and then spawn
)

(fn ConstructionScript)

(fn GetDatafromBank
  (params (MeshName :type Name%20%28by%20ref%29) (MaterialName :type Name%20%28by%20ref%29))
  (Utilities|FlowControl|Sequence
    (:then_0
      (bind _returnvalue (Utilities|GetDataTableRow (Variables|Default|GetStaticMeshBank) MeshName)
        (:then
          (LocalVariables|SetFoundStaticMesh (.StaticMesh (Utilities|Struct|BreakBGStaticMeshBank _returnvalue))))))
    (:then_1
      (bind _returnvalue_2 (Utilities|GetDataTableRow (Variables|Default|GetMaterialInstanceBank) MaterialName)
        (:then
          (LocalVariables|SetFoundMaterialInstance (.MaterialInstance (Utilities|Struct|BreakBGMaterialInstanceBank _returnvalue_2))))))
    (:then_2
      (return (LocalVariables|GetFoundStaticMesh) (LocalVariables|GetFoundMaterialInstance) (and (Utilities|IsValid (LocalVariables|GetFoundStaticMesh)) (Utilities|IsValid (LocalVariables|GetFoundMaterialInstance)))))))