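; BP_GameModeBase is the BattleGrids game mode, handling token actions server-side on requests from the PlayerController.
; It spawns tokens at a location by looking up their class by row name in the TokenDataBank table, then turns on physics simulation.
; Other events move an existing token to a tile location or set its mesh's physics and collision.
; A helper function returns a reference to the game mode itself.
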(event Custom|SpawnTokenOnTile
  (params (Location :type Vector) (RowName :type Name))
  ;[1 1 1] Called when a Drag & Drop operation is canceled (called by PlayerController)
  (bind _returnvalue (Utilities|GetDataTableRow (Variables|Config|GetTokenDataBank) RowName)
    (:then
      (bind _returnvalue_2 (Game|SpawnActorfromClass (.TokenClassReference (Utilities|Struct|BreakBGTokenBank _returnvalue)) (Math|Transform|MakeTransform Location "0, 0, 0" "1,1,1") "Undefined" self 0))
      (Physics|SetSimulatePhysics (Variables|/Script/BattleGrids.BGToken|GetStaticMeshComponent _returnvalue_2) true))
    (:RowNotFound
      (Development|PrintString "ERROR: Row Name does not exist in TokenDataBank"))))

(event Custom|MoveTokenToTile
  (params (Location :type Vector) (TokenToMove :type BG%20Token%20Object%20Reference))
  ;[1 1 1] Receives tile location vector and the token reference, and moves it, server-side (called by PlayerController)
  (Transformation|SetActorLocation TokenToMove Location false false))

(event Custom|SetTokenPhysicsAndCollision
  (params (Token :type BG%20Token%20Object%20Reference) (bPhysicsOn :type Boolean) (CollisionType :type ECollisionEnabled%20Enum :default "NoCollision"))
  (bind _staticmeshcomponent (Variables|/Script/BattleGrids.BGToken|GetStaticMeshComponent Token))
  ;[1 1 1] Enables physics and collision for a token, server-side (called by PlayerController)
  (Physics|SetSimulatePhysics _staticmeshcomponent bPhysicsOn)
  (Collision|SetCollisionEnabled _staticmeshcomponent CollisionType))

(fn ConstructionScript)

(fn GetGameModeReference
  (return self))